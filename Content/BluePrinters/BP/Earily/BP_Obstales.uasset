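; Obstacle actor that toggles a fire effect and notifies targets when its mesh is overlapped.
; The F key flip-flops between spawning a new Blueprint_Effect_Fire at the player's transform, stored in TargetFIre, and deactivating its particles and audio without destroying it.
; Actor overlap deactivates that stored fire, and ending the overlap reactivates it.
; Static mesh overlap adds the player character to Targets and sends them an interface message.
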(event `self.ReceiveActorBeginOverlap`
  (params (OtherActor :type "Actor Object Reference"))
  (`ActorComponent.Deactivate` (`/Game/StarterContent/Blueprints/Blueprint_Effect_Fire.P_Fire` (`self.TargetFIre`)))
  (`ActorComponent.Deactivate` (`/Game/StarterContent/Blueprints/Blueprint_Effect_Fire.Fire Audio` (`self.TargetFIre`))))

(event `self.ReceiveActorEndOverlap`
  (params (OtherActor :type "Actor Object Reference"))
  (`ActorComponent.Activate` (`/Game/StarterContent/Blueprints/Blueprint_Effect_Fire.Fire Audio` (`self.TargetFIre`)) false)
  (`ActorComponent.Activate` (`/Game/StarterContent/Blueprints/Blueprint_Effect_Fire.P_Fire` (`self.TargetFIre`)) false))

(event `Key|F`
  (params (Key :type "Key Structure"))
  (:`Pressed`
    (`/Engine/EditorBlueprintResources/StandardMacros.FlipFlop`
      (:`A`
        (bind _returnvalue (`|SpawnActorFromClass` "/Game/StarterContent/Blueprints/Blueprint_Effect_Fire.Blueprint_Effect_Fire_C" (`self.GetTransform` (`GameplayStatics.GetPlayerCharacter` 0)) "Undefined" "MultiplyWithRoot" null null))
        (set `self.TargetFIre` _returnvalue))
      (:`B`
        (`ActorComponent.Deactivate` (`/Game/StarterContent/Blueprints/Blueprint_Effect_Fire.Fire Audio` (`self.TargetFIre`)))
        (`ActorComponent.Deactivate` (`/Game/StarterContent/Blueprints/Blueprint_Effect_Fire.P_Fire` (`self.TargetFIre`)))))))

(event `self.StaticMesh.OnComponentBeginOverlap`
  (params (OverlappedComponent :type "PrimitiveComponent Object Reference") (OtherActor :type "Actor Object Reference") (OtherComp :type "PrimitiveComponent Object Reference") (OtherBodyIndex :type Integer) (bFromSweep :type Boolean) (SweepResult :type "HitResult Structure (by ref)"))
  (bind __targets (`self. Targets`))
  (`KismetArrayLibrary.Array_Add` __targets (`GameplayStatics.GetPlayerCharacter` 0))
  (message `/Game/BluePrinters/BP/Earily/BP_Interface_Cube.BP_Interface` __targets))

(fn `UserConstructionScript`)