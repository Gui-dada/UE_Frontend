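; BP_Func is a small actor Blueprint that exercises a custom function and shows its result on screen.
; On BeginPlay it calls NewFunction01 and prints the returned value.
; NewFunction01 raises the Addmin variable to a floor of ten, then returns it plus the input.
; Overlap, Tick and the construction script do nothing.
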(event `self.ReceiveBeginPlay`
  (bind _returnvalue (`self.NewFunction01` 1))
  (`KismetSystemLibrary.PrintString` (`KismetStringLibrary.Conv_IntToString` _returnvalue) true true (struct :`G` 0.66 :`B` 1.0 :`A` 1.0) 5.0))

(fn `NewFunction01`
  (params (var :type Integer))
  (returns (ReturnValue :type Integer))
  (locals (addmin :type Integer :default 5))
  (if (not (> (`local.addmin`) 10))
    (bind _output_get (set `local.addmin` 10)))
  (return (+ _output_get var)))

(fn `UserConstructionScript`)