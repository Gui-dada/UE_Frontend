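; BP_Runner is a player-controlled character with Enhanced Input movement, look, jump and an adjustable camera boom.
; BeginPlay adds the IMC_Runner mapping context, and movement follows control yaw, with control roll also passed to the direction vectors.
; ArmAdd and ArmDec print debug text and play timelines that change spring arm length by a fixed step on every update, so zoom distance depends on update count.
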(event `InputAction|ArmAdd`
  (params (Key :type "Key Structure"))
  ;[0.05127 0.05127 0.05127] TimeLineANDInput
  (:`Pressed`
    (`KismetSystemLibrary.PrintString` "加50")
    (`Timeline|AwayfromTimeline` :`NewTime` 0.25
      (:`Update`
        (set `SpringArmComponent.TargetArmLength` (+ (`SpringArmComponent.TargetArmLength` (`self.SpringArm`)) 50.0) (`self.SpringArm`))))))

(event `InputAction|ArmDec`
  (params (Key :type "Key Structure"))
  ;[0.05127 0.05127 0.05127] TimeLineANDInput
  (:`Pressed`
    (`KismetSystemLibrary.PrintString` "减50")
    (`Timeline|CloseToTimeline` :`NewTime` 0.25
      (:`Update`
        (set `SpringArmComponent.TargetArmLength` (- (`SpringArmComponent.TargetArmLength` (`self.SpringArm`)) 50.0) (`self.SpringArm`))))))

(event `self.ReceiveBeginPlay`
  (`EnhancedInputSubsystemInterface.AddMappingContext` (pcsubsystem `EnhancedInputLocalPlayerSubsystem` (`GameplayStatics.GetPlayerController` 0)) "/Game/BluePrinters/BP/Input/IMC_Runner.IMC_Runner" 0 (struct)))

(event `EnhancedInput|/Game/BluePrinters/BP/Input/Action/IAG_Move`
  (params (ActionValue :type "Vector2D Structure") (ElapsedSeconds :type "Float (double-precision)") (TriggeredSeconds :type "Float (double-precision)") (InputAction :type "InputAction Object Reference" :default "/Game/BluePrinters/BP/Input/Action/IAG_Move.IAG_Move"))
  (bind (_returnvalue_roll _returnvalue_pitch _returnvalue_yaw) (`KismetMathLibrary.BreakRotator` (`self.GetControlRotation`)))
  (bind (_returnvalue_roll_2 _returnvalue_pitch_2 _returnvalue_yaw_2) (`KismetMathLibrary.BreakRotator` (`self.GetControlRotation`)))
  (:`Triggered`
    (`self.AddMovementInput` (`KismetMathLibrary.GetRightVector` (`KismetMathLibrary.MakeRotator` _returnvalue_roll_2 0.0 _returnvalue_yaw_2)) ActionValue_X)
    (`self.AddMovementInput` (`KismetMathLibrary.GetForwardVector` (`KismetMathLibrary.MakeRotator` _returnvalue_roll 0.0 _returnvalue_yaw)) ActionValue_Y)))

(event `EnhancedInput|/Game/BluePrinters/BP/Input/Action/IAG_Lookat`
  (params (ActionValue :type "Vector2D Structure") (ElapsedSeconds :type "Float (double-precision)") (TriggeredSeconds :type "Float (double-precision)") (InputAction :type "InputAction Object Reference" :default "/Game/BluePrinters/BP/Input/Action/IAG_Lookat.IAG_Lookat"))
  (:`Triggered`
    (`self.AddControllerYawInput` ActionValue_X)
    (`self.AddControllerPitchInput` (* ActionValue_Y -1.0))))

(event `EnhancedInput|/Game/BluePrinters/BP/Input/Action/IAG_Jump`
  (params (ActionValue :type Boolean) (ElapsedSeconds :type "Float (double-precision)") (TriggeredSeconds :type "Float (double-precision)") (InputAction :type "InputAction Object Reference" :default "/Game/BluePrinters/BP/Input/Action/IAG_Jump.IAG_Jump"))
  (:`Started`
    (`self.Jump`))
  (:`Completed`
    (`self.StopJumping`)))

(fn `UserConstructionScript`)